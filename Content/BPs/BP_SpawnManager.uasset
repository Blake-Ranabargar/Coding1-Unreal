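; BP_SpawnManager spawns waves of BP_Enemy at the BP_SpawnPoint actors placed in the level.
; On BeginPlay, SpawnEnemies loops over every spawn point, giving each a weighted coin flip to spawn an enemy at its transform.
; NewWaveCheck counts living enemies and, when none remain, waits briefly before spawning the next wave.
; Debug print strings trace each step.
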(event Custom|Spawn%20Enemies
  (bind _outactors (Actor|GetAllActorsOfClass "/Game/BPs/BP_SpawnPoint.BP_SpawnPoint_C")) ; Get an Array of all Spawn Points Within The Level
  (for _array_element _outactors
    (Development|PrintString (Utilities|GetDisplayName _array_element))
    (if (Math|Random|RandomBoolwithWeight 0.5)
      (Game|SpawnActorfromClass "/Game/BPs/BP_Enemy.BP_Enemy_C" (Transformation|GetWorldTransform (Variables|/Game/BPs/BP_SpawnPoint.BP_SpawnPoint_C|GetDefaultSceneRoot _array_element)) "Undefined" "MultiplyWithRoot" 0 0)))
  (Development|PrintString "Finished With the For Each Loop for Spawn Enemies"))

(event Custom|NewWaveCheck
  (Development|PrintString "Was That the Last Enemy?")
  (bind _outactors (Actor|GetAllActorsOfClass "/Game/BPs/BP_Enemy.BP_Enemy_C"))
  (if (> (Utilities|Array|Length _outactors) 0)
    (Development|PrintString "You Were Not The Last One")
    (else
      (Development|PrintString "New Wave Incoming..." true true "(R=1.000000,G=0.071830,B=0.000000,A=1.000000)")
      (Utilities|FlowControl|Delay 3.0)
      (CallFunction|SpawnEnemies))))

(event EventBeginPlay
  (Development|PrintString "Spawn Manager Exists") ; Tell The Player That We Exist
  (CallFunction|SpawnEnemies))

(fn ConstructionScript)