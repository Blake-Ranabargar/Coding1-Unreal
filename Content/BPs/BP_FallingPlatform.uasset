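; Falling platform actor that drops after the player character steps into its trigger box, then returns to its starting transform.
; An overlap while ready starts a chain of delayed events: activate, fall by enabling physics simulation, then reset.
; Reset turns physics off and uses a timeline to lerp location and rotation from the fallen pose back to the one saved at BeginPlay.
; Each state swaps the platform material and the timeline's finish re-arms the trigger.
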(event OnComponentBeginOverlap(Box_Trigger)
  (params (OverlappedComponent :type Primitive%20Component%20Object%20Reference) (OtherActor :type Actor%20Object%20Reference) (OtherComp :type Primitive%20Component%20Object%20Reference) (OtherBodyIndex :type Integer) (bFromSweep :type Boolean) (SweepResult :type Hit%20Result%20Structure%20%28by%20ref%29))
  ;[0.15 0.02114 0.1019 0.5] Casting the overlap to the player BP/controller
  (Development|PrintString "Platform Trigger Activated")
  (if (Variables|Default|GetisReady)
    (Utilities|Casting|CastToBP_ThirdPersonCharacter_Custom OtherActor)
    (CallFunction|Activated)))

(event Custom|Activated
  ;[0.01776 0.15 0.04836 0.5] Begin Overlap Delay
  (Development|PrintString "Activated")
  (Variables|Default|SetisReady false)
  (Rendering|Material|SetMaterial (Variables|Default|GetPlatform) 0 "/Game/Materials/Platform/MI_Platform_Activated.MI_Platform_Activated")
  (Utilities|FlowControl|Delay (Variables|PlatformSettings|GetFall%20Delay%20Duration))
  (CallFunction|Falling))

(event Custom|Falling
  (bind _platform (Variables|Default|GetPlatform))
  ;[0.15 0 0.006467 0.5] Simulate physics and make the platform fall after a 1sec overlap
  (Development|PrintString "Falling")
  (Rendering|Material|SetMaterial _platform 0 "/Game/Materials/Platform/MI_Platform_Falling.MI_Platform_Falling")
  (Physics|SetSimulatePhysics _platform true)
  (Utilities|FlowControl|Delay 3.0)
  (CallFunction|Reseting))

(event Custom|reseting
  ;[0.15 0.131 0 0.5] Calling Reset Transform based on a timeline keyframe
  (Utilities|FlowControl|Delay 5.0)
  (Rendering|Material|SetMaterial (Variables|Default|GetPlatform) 0 "/Game/Materials/Platform/MI_Platform_Reseting.MI_Platform_Reseting")
  (Variables|Default|SetFallen%20Tranform (Transformation|GetWorldTransform (Variables|Default|GetPlatform)))
  (Physics|SetSimulatePhysics (Variables|Default|GetPlatform) false)
  (Development|PrintString "Reseting")
  (bind _falling_platform (Timeline|Timeline Play)
    (:Update
      (Transformation|SetWorldLocationAndRotation (Variables|Default|GetPlatform) (.location (Math|Transform|Lerp(Transform) (Variables|Default|GetFallen%20Tranform) (Variables|Default|GetOriginal%20Transform) _falling_platform)) (.rotation (Math|Transform|Lerp(Transform) (Variables|Default|GetFallen%20Tranform) (Variables|Default|GetOriginal%20Transform) _falling_platform)) false false))
    (:Finished
      (Variables|Default|SetisReady true)
      (Rendering|Material|SetMaterial (Variables|Default|GetPlatform) 0 "/Game/Materials/Platform/MI_Platform_Ready.MI_Platform_Ready"))))

(event EventBeginPlay
  ;[0 0.09769 0.15 0.5] Finiding and Setting the original Transform
  (Variables|Default|SetOriginal%20Transform (Transformation|GetWorldTransform (Variables|Default|GetPlatform))))

(fn ConstructionScript)